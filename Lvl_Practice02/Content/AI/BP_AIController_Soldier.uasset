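; AI controller for soldiers that sends the controlled pawn wandering between the waypoints it may use.
; On BeginPlay it gathers BP_Waypoint actors whose AllowedAccess contains its BP_AICharacter_Base pawn, shuffles them and moves to the first.
; Each completed move repeats this after a short delay, appending to Routes without emptying it, as the Clear node is unconnected.
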(event `self.ReceiveBeginPlay`
  (bind _routes (`self.Routes`))
  (add `self.ReceiveMoveCompleted` (delegate `MoveCompleted`))
  (bind _outactors (`GameplayStatics.GetAllActorsOfClass` "/Game/AI/Waypoints/BP_Waypoint.BP_Waypoint_C" :!label _label))
  (bind _asbp_aicharacter_base (cast `/Game/AI/BP_AICharacter_Base` (`self.K2_GetPawn`)))
  (for _array_element _outactors
    (if (!= (`KismetArrayLibrary.Array_Find` (`/Game/AI/Waypoints/BP_Waypoint.AllowedAccess` _array_element) _asbp_aicharacter_base) -1)
      (`KismetArrayLibrary.Array_Add` (`self.Routes`) _array_element)))
  (`KismetArrayLibrary.Array_Shuffle` _routes)
  (`self.MoveToActor` (`|GetArrayItem` _routes) -1.0 true true true null))

(event `MoveCompleted` :!signature `self.ReceiveMoveCompleted`
  (params (RequestID :type "AIRequestID Structure") (Result :type "EPathFollowingResult Enum" :default "Success"))
  (`KismetSystemLibrary.Delay` 3.0)
  (goto _label))

(fn `UserConstructionScript`)