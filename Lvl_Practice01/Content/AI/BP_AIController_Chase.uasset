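; AI controller that makes its pawn follow the player, aiming for a standoff point short of them along the line between the two.
; On Tick, throttled by a short Delay, it traces visibility from the pawn to that point.
; A hit switches the destination to a point beside the player, perpendicular to that line.
; MoveToLocation runs without pathfinding, so this trace-based sidestep is the only obstacle handling shown.
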(event `self.ReceiveTick`
  (params (DeltaSeconds :type "Float (single-precision)"))
  (bind _returnvalue (`self.K2_GetActorLocation` (`self.K2_GetPawn`)))
  (bind _returnvalue_2 (`self.K2_GetActorLocation` (`GameplayStatics.GetPlayerPawn` 0)))
  (bind _returnvalue_3 (`KismetMathLibrary.GetDirectionUnitVector` _returnvalue_2 _returnvalue))
  (bind _returnvalue_4 (+ _returnvalue_2 (* _returnvalue_3 300)))
  (`KismetSystemLibrary.Delay` 0.05)
  (bind (_outhit _returnvalue_5) (`KismetSystemLibrary.LineTraceSingle` _returnvalue _returnvalue_4 "TraceTypeQuery1"))
  (`self.MoveToLocation` (`KismetMathLibrary.SelectVector` (+ _returnvalue_2 (* (`KismetMathLibrary.GetRightVector` (`KismetMathLibrary.MakeRotFromX` _returnvalue_3)) -300)) _returnvalue_4 _returnvalue_5) -1.0 true false false true null))

(fn `UserConstructionScript`)