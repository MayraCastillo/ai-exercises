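; AI controller that keeps its pawn moving forward and turns it aside when something blocks the way.
; Tick passes through a one-second Delay, then runs a short visibility line trace ahead of the pawn.
; A hit sends the pawn to a point on its right, otherwise to a point straight ahead, using MoveToLocation without pathfinding.
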(event `self.ReceiveTick`
  (params (DeltaSeconds :type "Float (single-precision)"))
  (bind _returnvalue (`self.K2_GetPawn`))
  (bind _returnvalue_2 (`self.K2_GetActorLocation` (`self.K2_GetPawn`)))
  (bind _returnvalue_3 (+ _returnvalue_2 (* (`self.GetActorForwardVector` _returnvalue) 300)))
  (`KismetSystemLibrary.Delay` 1.0)
  (bind (_outhit _returnvalue_4) (`KismetSystemLibrary.LineTraceSingle` _returnvalue_2 _returnvalue_3 "TraceTypeQuery1"))
  (`self.MoveToLocation` (`KismetMathLibrary.SelectVector` (+ _returnvalue_2 (* (`self.GetActorRightVector` _returnvalue) 600)) _returnvalue_3 _returnvalue_4) -1.0 true false false true null))

(fn `UserConstructionScript`)